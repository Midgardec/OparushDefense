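; Bazooka tower Blueprint that handles the tower's flipbook animation and blast sound.
; Each Tick, it plays the shoot flipbook while shooting is allowed, rotated to match the sprite direction flag, and otherwise the idle flipbook.
; When Blasted is set, it clears the flag, plays an explosion sound, and either clears FinishedBlast or sets it after a delay.
; Targeting and distance-check fragments remain unconnected.
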(event `self.ReceiveTick`
  (params (DeltaSeconds :type "Float (single-precision)"))
  (bind _paperflipbook (`self.PaperFlipbook`))
  (`parent.ReceiveTick` DeltaSeconds)
  (`|ExecutionSequence`
    (:`then_0`
      (if (`self.bIsAllowedToShoot`)
        (`PaperFlipbookComponent.SetFlipbook` _paperflipbook "/Game/_Main/Sprites/Towers/BAZOOKA/Shoot_Bazooka.Shoot_Bazooka")
        (if (not (`self.bSpriteDirectionRight`))
          (`SceneComponent.K2_SetWorldRotation` _paperflipbook (struct :`Yaw` 90.0) false false)
          (else
            (`SceneComponent.K2_SetWorldRotation` _paperflipbook (struct :`Yaw` -90.0) false false)))
        (else
          (`PaperFlipbookComponent.SetFlipbook` (`self.PaperFlipbook`) "/Game/_Main/Sprites/Towers/BAZOOKA/Idle_bazooka.Idle_bazooka"))))
    (:`then_1`
      (if (`self.blasted`)
        (set `self.blasted` false)
        (`GameplayStatics.PlaySound2D` "/Game/_Main/Sounds/explodemini.explodemini" 0.5 1.0 0.0 null null)
        (if (`self.finished blast`)
          (set `self.finished blast` false)
          (else
            (`KismetSystemLibrary.Delay` 2.0)
            (set `self.finished blast` true)))))))

(event `self.PaperFlipbook.OnFinishedPlaying`)

(fn `UserConstructionScript`
  (`parent.UserConstructionScript`))