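; Player character Blueprint that puts up the Logo widget and handles pausing the game.
; BeginPlay creates the widget, stores it as UI and adds it to the player screen.
; Escape and P share one FlipFlop that alternates between pausing and unpausing.
; Tick checks whether castle health has reached zero but nothing follows the branch, and the overlap event is empty.
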(event `self.ReceiveBeginPlay`
  (bind _returnvalue (`|CreateWidget` "/Game/_Main/UI/Logo.Logo_C"))
  (bind _output_get (set `self.UI` _returnvalue))
  (`UserWidget.AddToPlayerScreen` _output_get 0))

(event `self.ReceiveTick`
  (params (DeltaSeconds :type "Float (single-precision)"))
  (if (<= (`self.CurrentCastleHealth`) 0.0)
    _))

(event `Key|Escape` :paused true
  (params (Key :type "Key Structure"))
  (:`Pressed`
    (`/Engine/EditorBlueprintResources/StandardMacros.FlipFlop` :!label _label
      (:`A`
        (`GameplayStatics.SetGamePaused` (`self.paused`)))
      (:`B`
        (`GameplayStatics.SetGamePaused` (`self.un paused`))))))

(event `Key|P` :paused true
  (params (Key :type "Key Structure"))
  (:`Pressed`
    (goto _label)))

(fn `UserConstructionScript`)