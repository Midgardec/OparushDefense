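; Minigun tower Blueprint that animates its Paper2D flipbook sprite according to its firing state.
; Each Tick runs the parent logic, then switches between the shoot and idle flipbooks based on IsAllowedToShoot.
; While shooting, SpriteDirectionRight flips the sprite between two opposite world rotations.
; The file contains no targeting or damage logic, and its finished-playing event is empty.
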(event `self.ReceiveTick`
  (params (DeltaSeconds :type "Float (single-precision)"))
  (bind _paperflipbook (`self.PaperFlipbook`))
  (`parent.ReceiveTick` DeltaSeconds)
  (if (`self.bIsAllowedToShoot`)
    (`PaperFlipbookComponent.SetFlipbook` _paperflipbook "/Game/_Main/Sprites/Towers/shooter/Shoot4.Shoot4")
    (if (not (`self.bSpriteDirectionRight`))
      (`SceneComponent.K2_SetWorldRotation` _paperflipbook (struct :`Yaw` 90.0) false false)
      (else
        (`SceneComponent.K2_SetWorldRotation` _paperflipbook (struct :`Yaw` -90.0) false false)))
    (else
      (`PaperFlipbookComponent.SetFlipbook` (`self.PaperFlipbook`) "/Game/_Main/Sprites/Towers/shooter/Idle3.Idle3"))))

(event `self.PaperFlipbook.OnFinishedPlaying`)

(fn `UserConstructionScript`
  (`parent.UserConstructionScript`))